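; BP_ChatMode is a game mode that sets up a turn-based host-versus-guest number game and relays chat messages.
; On BeginPlay it generates the target number and initializes each side's attempts and wins, the starting turn and a turn timer value.
; GotMessageFromClient forwards a message to every player controller through BP_Controller's GotBroadcast.
; Turn, timer and win logic are not implemented in this graph.
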(event Custom|GotMessageFromClient
  (params (Msg :type String))
  ;[0.15 0.15 0.15 0.5] PlayerController를가져와서 GetBroadcast
  (bind _outactors (Actor|GetAllActorsOfClass "/Script/Engine.PlayerController"))
  (for _array_element _outactors
    (bind _asbp_controller (Utilities|Casting|CastToBP_Controller _array_element))
    (Default|GotBroadcast _asbp_controller Msg)))

(event EventBeginPlay
  ;[0.15 0.15 0.15 0.5] 게임 초기화
  (bind _returnvalue (Class|NumberGenerator|GenerateNumber))
  (Variables|Default|SetTargetNumber _returnvalue)
  (Variables|Default|SetHostAttempts 3)
  (Variables|Default|SetGuestAttempts 3)
  (Variables|Default|SetbIsHostTurn true)
  (Variables|Default|SetTurnTimer 3e+01)
  (Variables|Default|SetHostWins 0)
  (Variables|Default|SetGuestWins 0))

(event EventTick
  (params (DeltaSeconds :type Float%20%28single-precision%29)))

(fn ConstructionScript)